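; Game instance Blueprint that runs an in-game radio, playing songs one after another.
; StartRadio initializes the radio, starts the first song and begins the wait loop.
; WaitSongEnd delays for the current song's duration, then plays the next song and calls itself again while ShouldPlay is true.
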(event Custom|WaitSongEnd
  (Utilities|FlowControl|Delay (Variables|/Script/Engine.SoundBase|GetDuration (Variables|Default|Get_CurrentSong)))
  (if (Variables|Default|Get_ShouldPlay)
    (Class|MyMusicManagerGameInstance|PlayNextSong)
    (CallFunction|WaitSongEnd)))

(fn StartRadio
  (Class|MyMusicManagerGameInstance|InitRadio)
  (Class|MyMusicManagerGameInstance|PlayNextSong)
  (CallFunction|WaitSongEnd))